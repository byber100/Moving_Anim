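; BP_P38 is a player-controlled P-38 plane pawn that flies forward continuously and fires rockets.
; Tick spins the left and right propeller meshes in opposite directions and feeds forward movement input scaled by the Boost value.
; Roll, Pitch and Yaw axes rotate the actor locally, scaled by frame time.
; Holding Boost raises thrust from half to full, and Fire spawns a BP_Rocket at the Arrow component's transform.
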(event EventTick
  (params (DeltaSeconds :type Float%20%28single-precision%29))
  ;[1 1 1] 프로펠러 회전
  (Transformation|AddLocalRotation (Variables|Default|GetSM_P38_Propeller_L) (Math|Rotator|MakeRotator (* (Utilities|Time|GetWorldDeltaSeconds) (Variables|속력|GetPropellerRotateSpeed)) 0.0 0.0) false false)
  (Transformation|AddLocalRotation (Variables|Default|GetSM_P38_Propeller_R) (Math|Rotator|MakeRotator (* (Utilities|Time|GetWorldDeltaSeconds) (Variables|속력|GetPropellerRotateSpeed) -1.0) 0.0 0.0) false false)
  (Pawn|Input|AddMovementInput (Transformation|GetActorForwardVector) (Variables|속력|GetBoost) false) ; 앞으로 전진
)

(event Input|ActionEvents|InputActionBoost
  (params (Key :type Key%20Structure :default "None"))
  (:Pressed
    (Variables|속력|SetBoost 1.0))
  (:Released
    (Variables|속력|SetBoost 0.5)))

(event Input|ActionEvents|InputActionFire
  (params (Key :type Key%20Structure :default "None"))
  (:Pressed
    (Game|SpawnActorfromClass "/Game/P38/BP_Rocket.BP_Rocket_C" (Transformation|GetWorldTransform (Variables|Default|GetArrow)) "Undefined" 0 0)))

(event Input|AxisEvents|InputAxisRoll
  (params (AxisValue :type Float%20%28single-precision%29))
  ;[1 1 1] 비행기 무빙 컨트롤
  (Transformation|AddActorLocalRotation (Math|Rotator|MakeRotator (* AxisValue (Variables|속력|GetRotateSpeed) (Utilities|Time|GetWorldDeltaSeconds)) 0.0 0.0) false false))

(event Input|AxisEvents|InputAxisPitch
  (params (AxisValue :type Float%20%28single-precision%29))
  ;[1 1 1] 비행기 무빙 컨트롤
  (Transformation|AddActorLocalRotation (Math|Rotator|MakeRotator 0.0 (* AxisValue (Variables|속력|GetRotateSpeed) (Utilities|Time|GetWorldDeltaSeconds)) 0.0) false false))

(event Input|AxisEvents|InputAxisYaw
  (params (AxisValue :type Float%20%28single-precision%29))
  ;[1 1 1] 비행기 무빙 컨트롤
  (Transformation|AddActorLocalRotation (Math|Rotator|MakeRotator 0.0 0.0 (* AxisValue (Variables|속력|GetRotateSpeed) (Utilities|Time|GetWorldDeltaSeconds))) false false))

(fn ConstructionScript)